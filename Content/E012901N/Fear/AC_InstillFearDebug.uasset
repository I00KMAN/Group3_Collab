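; Debug component that uses debug keys to test the fear system on enemies.
; H and J each send a fixed amount of fear, one fear type per key, to the AC_Fear component of every BP_DebugEnemy in the world.
; T runs a visualized box trace for pawns around the owner, ignoring the player pawn, and sends KillDebugMessage to hit actors that implement BPI_Fear.
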(event Input|KeyboardEvents|DebugKeyH
  (params (Key :type Key%20Structure :default "None") (ActionValue :type Input%20Action%20Value%20Structure))
  (:Pressed
    (bind _outactors (Actor|GetAllActorsOfClass "/Game/E012901N/Fear/BP_DebugEnemy.BP_DebugEnemy_C"))
    (for _array_element _outactors
      (Class|BPIFear|AddFear(Message) (Actor|GetComponentbyClass _array_element "/Game/E012901N/Fear/AC_Fear.AC_Fear_C") 15.0 "NewEnumerator0"))))

(event Input|KeyboardEvents|DebugKeyJ
  (params (Key :type Key%20Structure :default "None") (ActionValue :type Input%20Action%20Value%20Structure))
  (:Pressed
    (bind _outactors (Actor|GetAllActorsOfClass "/Game/E012901N/Fear/BP_DebugEnemy.BP_DebugEnemy_C"))
    (for _array_element _outactors
      (Class|BPIFear|AddFear(Message) (Actor|GetComponentbyClass _array_element "/Game/E012901N/Fear/AC_Fear.AC_Fear_C") 15.0 "NewEnumerator1"))))

(event Input|KeyboardEvents|DebugKeyT
  (params (Key :type Key%20Structure :default "None") (ActionValue :type Input%20Action%20Value%20Structure))
  (bind _returnvalue (Components|GetOwner))
  (bind _returnvalue_2 (Transformation|GetActorLocation _returnvalue))
  (:Pressed
    (bind _outhits (Class|KismetSystemLibrary|BoxTraceMultiforObjects _returnvalue_2 _returnvalue_2 "120.000000,120.000000,120.000000" "0, 0, 0" (Utilities|Array|MakeArray "ObjectTypeQuery3") false (Utilities|Array|MakeArray (Game|Player|GetPlayerPawn 0)) "ForDuration" true))
    (for _array_element _outhits
      (if (Utilities|DoesObjectImplementInterface (.HitActor (Collision|BreakHitResult _array_element)) "/Game/E012901N/Fear/BPI_Fear.BPI_Fear_C")
        (Class|BPIFear|Kill(Debug)(Message) (.HitActor (Collision|BreakHitResult _array_element)))))))