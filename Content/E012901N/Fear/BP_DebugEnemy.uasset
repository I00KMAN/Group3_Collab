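; BP_DebugEnemy is a debug enemy actor for exercising the fear system and its kill condition.
; On BeginPlay it initializes its ACFear component and binds to its can-be-killed event, then hands itself to the WBP_Fear widget for display.
; The event stores a Killable flag, and the debug Kill event destroys the actor only when that flag is set.
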(event `self.ReceiveBeginPlay`
  (bind _ac_fear (`self.AC_Fear`))
  (`/Game/E012901N/Fear/AC_Fear.Init` _ac_fear 1.0)
  (add `/Game/E012901N/Fear/AC_Fear.CanBeKilled` _ac_fear (delegate `Can Die?`))
  (bind _aswbp_fear (cast `/Game/E012901N/Fear/WBP_Fear` (`WidgetComponent.GetWidget` (`self.Widget`))))
  (`/Game/E012901N/Fear/WBP_Fear.Init` _aswbp_fear self))

(event `Can Die?`
  (params (`Killable?` :type Boolean))
  (set `self.Killable?` `Killable?`))

(event `/Game/E012901N/Fear/BPI_Fear.Kill(Debug)`
  (if (`self.Killable?`)
    (`self.K2_DestroyActor`)))

(fn `UserConstructionScript`)