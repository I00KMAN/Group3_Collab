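; Actor component that manages its owner's abilities, swapping the BPC_BaseAbility component and tracking active durations and cooldowns.
; ActivateHunter toggles Vision, messaging every BPI_MarkForHunted actor, and reads its duration from DT_Ability.
; A looping timer polls the expiry-time map, removes finished abilities and clears itself once empty.
; Only Vision has expiry logic, switching off and recording a cooldown timestamp; Teleport, Smoke and Hallucination branches are empty.
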(event `Active Ability`
  ; Checks to see if any abilities are active
  (bind _returnvalue (`KismetSystemLibrary.K2_SetTimerDelegate` (delegate `Check If Any Ability`) 0.08 true))
  (set `self.Active Ability Timer` _returnvalue))

(event `Check If Any Ability`
  (bind _abilityactive (`self.AbilityActive`))
  ; Checks to see if any abilities are active
  (if (`BlueprintMapLibrary.Map_IsNotEmpty` _abilityactive)
    (bind (_keypin _valuepin) (`|MapForEach` _abilityactive)
      (:`then`
        (if (>= (`KismetSystemLibrary.GetGameTimeInSeconds`) _valuepin)
          (switch `/Game/E012901N/E_Ability` _keypin
            (:`NewEnumerator0`
              _)
            (:`NewEnumerator1`
              _)
            (:`NewEnumerator2`
              _)
            (:`NewEnumerator3`
              (if (`self.VisionActive`)
                (`self.Activate Hunter`))))
          (`BlueprintMapLibrary.Map_Remove` (`self.AbilityActive`) _keypin))))
    (else
      (`KismetSystemLibrary.K2_ClearAndInvalidateTimerHandle` (`self.Active Ability Timer`)))))

(event `Activate Hunter`
  (if (`self.VisionActive`)
    (bind _outactors (`GameplayStatics.GetAllActorsWithInterface` "/Game/n015382m/BPI_MarkForHunted.BPI_MarkForHunted_C"))
    (for _array_element _outactors
      (message `/Game/n015382m/BPI_MarkForHunted.Hunted` _array_element false))
    (set `self.VisionActive` false)
    (bind ((`Cooldown_2_BB66CFA64A14BBF093D91A9A2DF392B4` _cooldown) (`Length_4_A4EC643849EA160D505607AA5B6807F1` _length)) (break `/Game/E012901N/S_AbilityInfo` (stale _returnvalue)))
    (`self.Cooldown` "NewEnumerator3" _cooldown)
    (else
      (bind _outactors_2 (`GameplayStatics.GetAllActorsWithInterface` "/Game/n015382m/BPI_MarkForHunted.BPI_MarkForHunted_C"))
      (for _array_element_2 _outactors_2
        (message `/Game/n015382m/BPI_MarkForHunted.Hunted` _array_element_2 true))
      (set `self.VisionActive` true)
      (bind _returnvalue (`|GetDataTableRow` "/Game/E012901N/DT_Ability.DT_Ability" "Vision")
        (:`then`
          (`BlueprintMapLibrary.Map_Add` (`self.AbilityActive`) "NewEnumerator3" (+ (`KismetSystemLibrary.GetGameTimeInSeconds`) _length))
          (`self.Active Ability`))))))

(event `/Game/L011605n/BPI_Ability.Activate/Deactivate`
  (params (`To Activate` :type "/Game/L011605n/BPC_BaseAbility Class Reference"))
  (bind _returnvalue (`self.GetOwner`))
  (for _array_element (`Actor.K2_GetComponentsByClass` (`self.GetOwner`) "/Game/L011605n/BPC_BaseAbility.BPC_BaseAbility_C")
    (message `/Game/L011605n/BPI_PlayerCharacter.Destroy Comp` _returnvalue _array_element))
  (`|AddComponentByClass` _returnvalue `To Activate` self))

(fn `Cooldown`
  (params (Ability :type "/Game/E012901N/E_Ability Enum" :default "NewEnumerator0") (CooldownTime :type "Float (double-precision)"))
  (`BlueprintMapLibrary.Map_Add` (`self.CooldownMap`) Ability (+ (`KismetSystemLibrary.GetGameTimeInSeconds`) CooldownTime)))