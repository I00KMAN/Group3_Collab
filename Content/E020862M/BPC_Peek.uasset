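; Player component that lets a crouched, non-tilting character raise the first-person camera to peek over cover while the peek input is held.
; A forward trace finds the obstacle, a raised trace confirms clearance above it, and a downward sphere trace finds its top to size the camera offset.
; Peek state reaches the character through interface messages, and releasing the input reverses the stored offset.
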(event `self.ReceiveBeginPlay`
  (bind _playercharacter (message `/Game/L011605n/BPI_PlayerCharacter.GetPlayerCharacterRef` (`self.GetOwner`)))
  (bind _output_get (set `self.Player Character` _playercharacter))
  (set `self.Player Camera` (`/Game/FirstPerson/Blueprints/BP_FirstPersonCharacter.FirstPersonCamera` _output_get)))

(event `EnhancedInput|/Game/Input/Actions/IA_Peek`
  (params (ActionValue :type Boolean) (ElapsedSeconds :type "Float (double-precision)") (TriggeredSeconds :type "Float (double-precision)") (InputAction :type "InputAction Object Reference" :default "/Game/Input/Actions/IA_Peek.IA_Peek"))
  (:`Started`
    (if (`Character.bIsCrouched` (`self.Player Character`)) :!label _label
      (`self.HandlePeek` true)))
  (:`Ongoing`
    (goto _label))
  (:`Canceled`
    (if (`self.IsPeeking`) :!label _label_2
      (`self.HandlePeek` false)))
  (:`Completed`
    (goto _label_2)))

(fn `HandlePeek`
  (params (CanPeek :type Boolean))
  (locals (CurrentEyeHeight :type "Float (double-precision)") (CurrentEyeLocation :type "Vector Structure"))
  (bind _player_camera (`self.Player Camera`))
  (bind _player_camera_2 (`self.Player Camera`))
  (bind _currenteyelocation (`local.CurrentEyeLocation`))
  (bind _returnvalue (`SceneComponent.GetForwardVector` _player_camera_2))
  (bind _returnvalue_2 (`SceneComponent.K2_GetComponentLocation` _player_camera_2))
  (bind _returnvalue_3 (`KismetMathLibrary.MakeVector` (.x _currenteyelocation) (.y _currenteyelocation) (+ (.z _currenteyelocation) (`self.MaxPeekHeight`))))
  (bind _returnvalue_4 (`KismetMathLibrary.MakeVector` (.x _returnvalue_2) (.y _returnvalue_2) (+ (.z _returnvalue_2) (`self.MaxPeekHeight`))))
  (if (`/Game/FirstPerson/Blueprints/BP_FirstPersonCharacter.isTilting` (`self.Player Character`))
    _
    (elif CanPeek
      (bind (_outhit _returnvalue_5) (`KismetSystemLibrary.LineTraceSingle` :`Start` _returnvalue_2 :`End` (+ _returnvalue_2 (* _returnvalue (`self.MaxCanPeekDistance`))) :`TraceChannel` "TraceTypeQuery1" :`DrawDebugType` "ForDuration"))
      (if _returnvalue_5
        (bind (_bblockinghit _binitialoverlap _time _distance _location) (`GameplayStatics.BreakHitResult` _outhit))
        (set `local.CurrentEyeHeight` (.z _location))
        (set `local.CurrentEyeLocation` _location)
        (bind (_outhit_2 _returnvalue_6) (`KismetSystemLibrary.LineTraceSingle` :`Start` _returnvalue_4 :`End` (+ _returnvalue_4 (* _returnvalue (`self.MaxDistanceOverhead`))) :`TraceChannel` "TraceTypeQuery1" :`DrawDebugType` "ForDuration"))
        (if (not _returnvalue_6)
          (bind (_outhit_3 _returnvalue_7) (`KismetSystemLibrary.SphereTraceSingle` :`Start` _returnvalue_3 :`End` (+ _returnvalue_3 (* (* (`KismetMathLibrary.Vector_Up`) -1.0) (`KismetMathLibrary.VSize` (- _returnvalue_4 _currenteyelocation)))) :`Radius` 2.0 :`TraceChannel` "TraceTypeQuery1" :`DrawDebugType` "ForDuration"))
          (if _returnvalue_7
            (bind _returnvalue_8 (`KismetMathLibrary.MakeVector` (.x (`self.CameraPeekOffset`)) (.y (`self.CameraPeekOffset`)) (+ (.z (- (`.Location` (`GameplayStatics.BreakHitResult` _outhit_3)) (`SceneComponent.K2_GetComponentLocation` _player_camera))) (.z (`self.CameraPeekOffset`)))))
            (set `self.CurentCameraOffsetValue` _returnvalue_8)
            (`SceneComponent.K2_AddLocalOffset` _player_camera _returnvalue_8 false false)
            (bind _output_get (set `self.IsPeeking` true))
            (message `/Game/L011605n/BPI_PlayerCharacter.ISetPeeking` (`self.Player Character`) _output_get)
            (`KismetSystemLibrary.PrintString` "Peeking")))
        (else
          (set `local.CurrentEyeHeight` 0.0)
          (set `local.CurrentEyeLocation` (0.0 0.0 0.0))))
      (else
        (`KismetSystemLibrary.PrintString` "Not Peeking")
        (bind _output_get_2 (set `self.IsPeeking` false))
        (message `/Game/L011605n/BPI_PlayerCharacter.ISetPeeking` (`self.Player Character`) _output_get_2)
        (`SceneComponent.K2_AddLocalOffset` (`self.Player Camera`) (* (`self.CurentCameraOffsetValue`) -1.0) false false)))))