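; AI controller that runs the BT_BaseAI behavior tree and feeds it perception results through the Blackboard.
; On each perception update, it asks the sensed actor for a player character reference through a message call.
; A valid reference becomes PlayerTarget; otherwise it clears PlayerTarget and stores the stimulus location as TargetLocation.
; The stimulus's sensed-or-lost state is not checked, and GetAICharacter is an empty stub.
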(event `self.ReceiveBeginPlay`
  (`self.RunBehaviorTree` "/Game/L011605n/AI/BT_BaseAI.BT_BaseAI"))

(event `self.AIPerception.OnTargetPerceptionUpdated`
  (params (Actor :type "Actor Object Reference") (Stimulus :type "AIStimulus Structure"))
  (bind _playercharacter (message `/Game/L011605n/BPI_PlayerCharacter.GetPlayerCharacterRef` Actor))
  (`/Engine/EditorBlueprintResources/StandardMacros.IsValid` _playercharacter
    (:`Is Valid`
      (`KismetSystemLibrary.PrintString` "sensed")
      (bind _output_get (set `self.Player Character` _playercharacter))
      (`BlackboardComponent.SetValueAsObject` (`self.Blackboard`) "PlayerTarget" _output_get))
    (:`Is Not Valid`
      (`BlackboardComponent.ClearValue` (`self.Blackboard`) "PlayerTarget")
      (`BlackboardComponent.SetValueAsVector` (`self.Blackboard`) "TargetLocation" (`.StimulusLocation` (break `AIStimulus` Stimulus)))
      (`KismetSystemLibrary.PrintString` "not"))))

(fn `GetAICharacter`
  (returns (`AI Character` :type "/Game/L011605n/AI/BP_AICharacter Object Reference"))
  (return null))

(fn `UserConstructionScript`)