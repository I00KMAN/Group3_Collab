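; BP_AICharacter is an AI-controlled character that cycles through a set of patrol locations.
; On BeginPlay it copies its patrol points from the linked PatrolActor's OutputPatrolLocations.
; UpdatePatrolPoint advances the index, wraps to the first point after the last, and writes the new target to the AI controller's TargetLocation Blackboard key.
; Two getter functions expose the patrol points and the character itself.
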(event `self.ReceiveBeginPlay`
  (set `self.PatrolPoints` (`/Game/L011605n/AI/BP_PatrolCycle.OutputPatrolLocations` (`self.PatrolActor`))))

(event `/Game/L011605n/AI/BPI_AI.UpdatePatrolPoint`
  (bind _result (`/Engine/EditorBlueprintResources/StandardMacros.IncrementInt` (`self.PatrolPointIndex`))
    (:`  `
      (bind _returnvalue (select `bool` (> _result (- (`KismetArrayLibrary.Array_Length` (`self.PatrolPoints`)) 1)) :`false` _result))
      (set `self.PatrolPointIndex` _returnvalue)
      (bind _output_get (set `self.CurrentTarget` (`|GetArrayItem` (`self.PatrolPoints`) _returnvalue)))
      (`BlackboardComponent.SetValueAsVector` (`AIController.Blackboard` (`AIBlueprintHelperLibrary.GetAIController` self)) "TargetLocation" _output_get))))

(fn `Get Patrol Points`
  (returns (Points :type "Array of Vector Structure"))
  (return (`self.PatrolPoints`)))

(fn `GetAICharacter`
  (returns (`AI Character` :type "/Game/L011605n/AI/BP_AICharacter Object Reference"))
  (return self))

(fn `UserConstructionScript`)