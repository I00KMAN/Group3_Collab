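; BPC_Interact is a player interaction component with an unfinished teleport ability.
; On BeginPlay it caches the player character through a message call to its owner.
; The IA_Ability input event is empty, and the teleport logic is disconnected, so it never runs.
; That unused logic capsule-traces forward from the first-person camera to find a location, then moves the character there.
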(event `self.ReceiveBeginPlay`
  ; BeginPlay
  (bind _playercharacter (message `/Game/L011605n/BPI_PlayerCharacter.GetPlayerCharacterRef` (`self.GetOwner`)))
  (set `self.Player Character` _playercharacter))

(event `EnhancedInput|/Game/Input/Actions/IA_Ability`
  (params (ActionValue :type Boolean) (ElapsedSeconds :type "Float (double-precision)") (TriggeredSeconds :type "Float (double-precision)") (InputAction :type "InputAction Object Reference" :default "/Game/Input/Actions/IA_Ability.IA_Ability"))
  ; Ability (Teleport for Now)
)