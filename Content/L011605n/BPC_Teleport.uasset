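; Teleport ability component that moves the player to an aimed surface or perch point when off cooldown.
; Priming capsule-traces forward from the first-person camera over the ability's range, ignoring the occupied perch, then snaps to a hit perch's origin or shows a short-lived decal at the impact.
; Using the ability teleports without sweep to that stored location, records the perch and starts the cooldown through the ability manager.
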(event `EnhancedInput|/Game/IA_PrimeAbility`
  (params (ActionValue :type Boolean) (ElapsedSeconds :type "Float (double-precision)") (TriggeredSeconds :type "Float (double-precision)") (InputAction :type "InputAction Object Reference" :default "/Game/IA_PrimeAbility.IA_PrimeAbility"))
  (bind _returnvalue (`SceneComponent.GetForwardVector` (`self.First Person Camera`)))
  (bind _returnvalue_2 (`SceneComponent.K2_GetComponentLocation` (`self.First Person Camera`)))
  ; Input
  (:`Triggered`
    ; Checking if the ability is useable
    (if (`self.Cooled Down?`)
      (bind (_outhit _returnvalue_3) (`KismetSystemLibrary.CapsuleTraceSingleForObjects` (+ _returnvalue_2 (* _returnvalue 50.0)) (+ _returnvalue_2 (* _returnvalue (`.Range_16_C9F224434B2107C7AC12FD93EB9508E4` (break `/Game/E012901N/S_AbilityInfo` (`self.AbilityInfo`))))) 34.0 34.0 (`|MakeArray` "ObjectTypeQuery8" "ObjectTypeQuery1" :!type "EObjectTypeQuery Enum") false (`|MakeArray` (`self.HoveredPerchPoint`)) "ForDuration" true (struct :`R` 1.0 :`A` 1.0) (struct :`G` 1.0 :`A` 1.0) 0.2))
      ; Is valid TP surface
      (bind _output_get (set `self.ValidTP` _returnvalue_3))
      (if _output_get
        (bind (_bblockinghit _binitialoverlap _time _distance _location _impactpoint _normal _impactnormal _physmat _hitactor) (`GameplayStatics.BreakHitResult` _outhit))
        ; Is it a perch point?
        (if (== _hitactor "/Game/BP_PerchPoint.BP_PerchPoint_C")
          ; Set teleport location to perch point and store perch point ref
          (`/Engine/EditorBlueprintResources/StandardMacros.IsValid` _hitactor
            (:`Is Valid`
              (bind _output_get_2 (set `self.PerchToIgnore` _hitactor))
              (set `self.TeleportLocation` (`Actor.K2_GetActorLocation` _output_get_2)))
            (:`Is Not Valid`
              (set `self.PerchToIgnore` null)))
          (else
            ; Set teleport location to marker and clear perch point
            (bind _output_get_3 (set `self.TeleportLocation` _location))
            (set `self.PerchToIgnore` null)
            ; Add marker
            (bind _returnvalue_4 (`GameplayStatics.SpawnDecalAtLocation` "/Game/L011605n/M_TPDecal.M_TPDecal" (50.0 50.0 50.0) _output_get_3 (`KismetMathLibrary.Conv_VectorToRotator` _normal) 0.1))
            (`DecalComponent.SetFadeOut` _returnvalue_4 0.0 0.1 true)))))))

(event `EnhancedInput|/Game/IA_UseAbillity`
  (params (ActionValue :type Boolean) (ElapsedSeconds :type "Float (double-precision)") (TriggeredSeconds :type "Float (double-precision)") (InputAction :type "InputAction Object Reference" :default "/Game/IA_UseAbillity.IA_UseAbillity"))
  (:`Started`
    ; Can Teleport?
    (if (and (`self.Cooled Down?`) (`self.ValidTP`))
      ; Teleport to desired location
      (`Actor.K2_SetActorLocation` (`self.Player Character`) (`self.TeleportLocation`) false true)
      (set `self.HoveredPerchPoint` (`self.PerchToIgnore`))
      (`/Game/E012901N/AC_AbilityManager.Cooldown` (`self.AbilityManager`) "NewEnumerator0" (`.Cooldown_2_BB66CFA64A14BBF093D91A9A2DF392B4` (break `/Game/E012901N/S_AbilityInfo` (`self.AbilityInfo`)))))))