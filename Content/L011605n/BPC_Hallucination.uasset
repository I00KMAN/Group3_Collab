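; Hallucination ability component that lets the player inflict a hallucination on a targeted actor through its AC_Fear component.
; While priming off cooldown, a camera-based capsule trace finds a Destructible-type object, and a line trace rejects it if world geometry blocks it.
; Using the ability on a valid target sends the hallucination amount and duration from AbilityInfo, then starts the cooldown through AbilityManager.
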(event `EnhancedInput|/Game/IA_PrimeAbility`
  (params (ActionValue :type Boolean) (ElapsedSeconds :type "Float (double-precision)") (TriggeredSeconds :type "Float (double-precision)") (InputAction :type "InputAction Object Reference" :default "/Game/IA_PrimeAbility.IA_PrimeAbility"))
  (bind _returnvalue (* (`SceneComponent.GetForwardVector` (`self.First Person Camera`)) 50.0))
  (bind _returnvalue_2 (+ (`SceneComponent.K2_GetComponentLocation` (`self.First Person Camera`)) _returnvalue))
  (:`Triggered`
    (if (`self.Cooled Down?`)
      (bind (_outhit _returnvalue_3) (`KismetSystemLibrary.CapsuleTraceSingleForObjects` :`Start` _returnvalue_2 :`End` (* _returnvalue (`.Range_16_C9F224434B2107C7AC12FD93EB9508E4` (break `/Game/E012901N/S_AbilityInfo` (`self.AbilityInfo`)))) :`Radius` 50.0 :`HalfHeight` 10.0 :`ObjectTypes` (`|MakeArray` "ObjectTypeQuery6" :!type "EObjectTypeQuery Enum") :`DrawDebugType` "ForDuration"))
      (if _returnvalue_3
        (bind (_bblockinghit _binitialoverlap _time _distance _location _impactpoint _normal _impactnormal _physmat _hitactor) (`GameplayStatics.BreakHitResult` _outhit))
        (bind (_outhit_2 _returnvalue_4) (`KismetSystemLibrary.LineTraceSingleForObjects` :`Start` _returnvalue_2 :`End` _location :`ObjectTypes` (`|MakeArray` "ObjectTypeQuery1" "ObjectTypeQuery2" :!type "EObjectTypeQuery Enum") :`DrawDebugType` "ForDuration"))
        (if (== _returnvalue_4 false)
          (set `self.CurrentTarget` _hitactor)
          (else
            (set `self.CurrentTarget` null :!label _label)))
        (else
          (goto _label))))))

(event `EnhancedInput|/Game/IA_UseAbillity`
  (params (ActionValue :type Boolean) (ElapsedSeconds :type "Float (double-precision)") (TriggeredSeconds :type "Float (double-precision)") (InputAction :type "InputAction Object Reference" :default "/Game/IA_UseAbillity.IA_UseAbillity"))
  (bind _currenttarget (`self.CurrentTarget`))
  (bind ((`Cooldown_2_BB66CFA64A14BBF093D91A9A2DF392B4` _cooldown) (`Length_4_A4EC643849EA160D505607AA5B6807F1` _length) (`Value_18_0798080B4164E4101CE5409FB041BA8C` _value)) (break `/Game/E012901N/S_AbilityInfo` (`self.AbilityInfo`)))
  (:`Started`
    (`/Engine/EditorBlueprintResources/StandardMacros.IsValid` _currenttarget
      (:`Is Valid`
        (message `/Game/E012901N/Fear/BPI_Fear.Hallucination` (`Actor.GetComponentByClass` _currenttarget "/Game/E012901N/Fear/AC_Fear.AC_Fear_C") _value _length)
        (`/Game/E012901N/AC_AbilityManager.Cooldown` (`self.AbilityManager`) "NewEnumerator2" _cooldown)))))