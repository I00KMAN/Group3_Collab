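; BPC_BaseAbility is a base component for player abilities that supplies shared references, ability data and a cooldown check.
; On BeginPlay it caches the player character, first-person camera and AC_AbilityManager, then loads its DT_Ability row using the Ability enum as the row name.
; CooledDown compares game time with the expiry stored in the manager's CooldownMap, removing expired entries and treating missing ones as ready.
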(event `self.ReceiveBeginPlay`
  ; BeginPlay
  (bind _playercharacter (message `/Game/L011605n/BPI_PlayerCharacter.GetPlayerCharacterRef` (`self.GetOwner`)))
  (bind _output_get (set `self.Player Character` _playercharacter))
  (set `self.First Person Camera` (`/Game/FirstPerson/Blueprints/BP_FirstPersonCharacter.FirstPersonCamera` _output_get))
  (set `self.AbilityManager` (`Actor.GetComponentByClass` _playercharacter "/Game/E012901N/AC_AbilityManager.AC_AbilityManager_C"))
  (bind _returnvalue (`|GetDataTableRow` "/Game/E012901N/DT_Ability.DT_Ability" (`KismetStringLibrary.Conv_StringToName` (`|GetEnumeratorNameAsString` (`self.Ability`))))
    (:`then`
      (set `self.AbilityInfo` _returnvalue))))

(fn `Cooled Down?`
  (returns (Yes :type Boolean))
  (bind (_value _returnvalue) (`BlueprintMapLibrary.Map_Find` (`/Game/E012901N/AC_AbilityManager.CooldownMap` (`self.AbilityManager`)) (`self.Ability`)))
  (if _returnvalue
    (if (>= (`KismetSystemLibrary.GetGameTimeInSeconds`) _value)
      (`BlueprintMapLibrary.Map_Remove` (`/Game/E012901N/AC_AbilityManager.CooldownMap` (`self.AbilityManager`)) (`self.Ability`))
      (return true)
      (else
        (return false)))
    (else
      (return true))))